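; BP_ZonaMuerte is a death zone that reacts when any actor overlaps its Box.
; On overlap it sends CheckpointMessage to that actor, presumably to return it to a checkpoint, and plays a death sound.
; It increments a death counter stored on the zone and prints a mocking Spanish on-screen message with the count, plus an extra taunt at exactly five deaths.
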(event `self.Box.OnComponentBeginOverlap`
  (params (OverlappedComponent :type "PrimitiveComponent Object Reference") (OtherActor :type "Actor Object Reference") (OtherComp :type "PrimitiveComponent Object Reference") (OtherBodyIndex :type Integer) (bFromSweep :type Boolean) (SweepResult :type "HitResult Structure (by ref)"))
  (message `/Game/Interfaces/BPI_Checkpoint.Checkpoint` OtherActor)
  (`GameplayStatics.PlaySound2D` "/Game/TileSet/Assets/Musica/DeadSound.DeadSound" 1.0 1.0 0.0 null null)
  (bind _output_get (set `self.Cantidad de muertes` (+ (`self.Cantidad de muertes`) 1)))
  (`KismetSystemLibrary.PrintString` (`KismetStringLibrary.Concat_StrStr` "En serio moriste? eso que esta facil. \n" "Ya moriste: " (`KismetStringLibrary.Conv_IntToString` _output_get) " veces.") true true (struct :`R` 0.117298 :`G` 1.0 :`B` 0.058977 :`A` 1.0) 4.0)
  (if (== (`self.Cantidad de muertes`) 5)
    (`KismetSystemLibrary.PrintString` "Ya llegaste a 5 muertes? son 3 niveles nomas, proba el candy crush" true true (struct :`R` 0.117298 :`G` 1.0 :`B` 0.058977 :`A` 1.0) 4.0)))

(fn `UserConstructionScript`)